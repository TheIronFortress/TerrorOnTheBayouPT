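; A simple danger indicator that points toward an enemy and resizes according to that enemy's closeness value.
; On BeginPlay it loops over actors tagged "Enemy", keeping only the last one as its tracked target.
; Each tick it adds a LookAt rotation to Origin, using its up vector as the aim axis.
; It also scales Base uniformly by the result of BP_Enemy's CalculateCloseVolume.
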(event EventBeginPlay
  (bind _outactors (Actor|GetAllActorswithTag "Enemy"))
  (for _array_element _outactors
    (Variables|Default|SetEnemyRef _array_element)))

(event EventTick
  (params (DeltaSeconds :type Float%20%28single-precision%29))
  (bind _origin (Variables|Default|GetOrigin))
  (Utilities|IsValid (Variables|Default|GetEnemyRef)
    (:Is%20Valid
      (Transformation|AddWorldRotation _origin (.rotation (Class|KismetAnimationLibrary|Lookat (Transformation|GetWorldTransform _origin) (Transformation|GetActorLocation (Variables|Default|GetEnemyRef)) (Math|Vector|GetUpVector _origin) false "0, 0, 0" 0.0)) false false)
      (bind _asbp_enemy (Utilities|Casting|CastToBP_Enemy (Variables|Default|GetEnemyRef)))
      (Transformation|SetRelativeScale3D (Variables|Default|GetBase) (Math|Conversions|ToVector(Float) (Default|CalculateCloseVolume _asbp_enemy))))))

(fn ConstructionScript)