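; Monster enemy AI that roams around the player, chases within sense range and damages in attack range on a cooldown.
; Tick runs a Wander/Confuse/Pursuit state machine; losing the player leads to a last-known position, then a confused pause.
; Movement is swept forward steps with interpolated yaw, without navmesh.
; It also drives ambient sound parameters: closeness volume from distance, chase volume that ramps up during pursuit and never decreases.
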(event EventBeginPlay
  (bind (_x _y) (CallFunction|GenerateWanderLocation))
  (Utilities|FlowControl|Sequence
    (:then_0
      (bind _returnvalue (Actor|GetActorOfClass "/Script/Engine.AmbientSound"))
      (Variables|Default|SetAmbientSoundRef _returnvalue))
    (:then_1
      (bind _outactors (Actor|GetAllActorswithTag "Player"))
      (for _array_element _outactors
        (Variables|Default|SetPlayerRef _array_element)))
    (:then_2
      (Variables|Default|SetTargetLocation (Math|Vector|MakeVector _x _y 0.0)))))

(event EventTick
  (params (DeltaSeconds :type Float%20%28single-precision%29))
  (CallFunction|CheckMusic)
  (CallFunction|CheckSense)
  (CallFunction|CheckAttack)
  (switch Utilities|FlowControl|Switch|SwitchonE_EnemyState (Variables|Default|GetCurrentState)
    (:NewEnumerator0
      (CallFunction|HandleWander))
    (:NewEnumerator1
      (CallFunction|HandleConfuse))
    (:NewEnumerator2
      (CallFunction|HandlePursuit)))
  (CallFunction|MoveTowardTarget))

(fn ConstructionScript)

(fn HandleWander
  (bind (_x _y) (CallFunction|GenerateWanderLocation))
  (if (<= (Math|Vector|VectorLength (- (Transformation|GetActorLocation) (Variables|Default|GetTargetLocation))) (Variables|Default|GetNavigationTolerance))
    ;[0.4115 0.4115 0.4115] Set New Wander Target
    (Variables|Default|SetTargetLocation (Math|Vector|MakeVector _x _y 0.0))))

(fn HandleConfuse
  (if (<= (Variables|Default|GetConfuseTimer) 0.0)
    (Variables|Default|SetCurrentState "NewEnumerator0")
    (else
      (Variables|Default|SetConfuseTimer (- (Variables|Default|GetConfuseTimer) (Utilities|Time|GetWorldDeltaSeconds))))))

(fn HandlePursuit
  (if (<= (CallFunction|GetDistancetoPlayer) (Variables|Default|GetSenseRange))
    (Variables|Default|SetTargetLocation (Transformation|GetActorLocation (Variables|Default|GetPlayerRef)))
    (elif (<= (CallFunction|GetDistancetoTarget) (Variables|Default|GetNavigationTolerance))
      (Variables|Default|SetConfuseTimer (Variables|Default|GetMaxConfuseDelay))
      (Variables|Default|SetCurrentState "NewEnumerator1"))))

(fn MoveTowardTarget
  (Transformation|SetActorRotation (Math|Rotator|MakeRotator 0.0 0.0 (.yaw (Math|Interpolation|RInterpTo (Transformation|GetActorRotation) (Math|Rotator|FindLookatRotation (Transformation|GetActorLocation) (Variables|Default|GetTargetLocation)) (Utilities|Time|GetWorldDeltaSeconds) (Variables|Default|GetTurnSpeed)))))
  (Transformation|SetActorLocation (+ (Transformation|GetActorLocation) (* (Transformation|GetActorForwardVector) (Utilities|Time|GetWorldDeltaSeconds) (Utilities|Select :Index (Variables|Default|GetCurrentState) :NewEnumerator0 (Variables|Default|GetWanderSpeed) :NewEnumerator1 0.0 :NewEnumerator2 (Variables|Default|GetPursuitSpeed)))) true false))

(fn CheckSense
  (if (<= (CallFunction|GetDistancetoPlayer) (Variables|Default|GetSenseRange))
    (Variables|Default|SetCurrentState "NewEnumerator2")))

(fn CheckAttack
  (if (<= (CallFunction|GetDistancetoPlayer) (Variables|Default|GetAttackRange))
    (if (<= (Variables|Default|GetAttackResetTimer) 0.0)
      (Variables|Default|SetAttackResetTimer (Variables|Default|GetMaxAttackResetTime))
      (Audio|PlaySound2D "/Game/Audio/Cues/SC_MonsterAttack.SC_MonsterAttack" 1.0 1.0 0.0 0 0)
      (Class|IDamageAble|TakeDamage(Message) (Variables|Default|GetPlayerRef))
      (Development|PrintString "Attacked!")
      (else
        (Variables|Default|SetAttackResetTimer (- (Variables|Default|GetAttackResetTimer) (Utilities|Time|GetWorldDeltaSeconds)))))))

(fn GetDistancetoPlayer
  (return (Math|Vector|VectorLength (- (Transformation|GetActorLocation (Variables|Default|GetPlayerRef)) (Transformation|GetActorLocation)))))

(fn GetDistancetoTarget
  (return (Math|Vector|VectorLength (- (Variables|Default|GetTargetLocation) (Transformation|GetActorLocation)))))

(fn CheckMusic
  (bind _ambientsoundref (Variables|Default|GetAmbientSoundRef))
  (bind _audiocomponent (Variables|/Script/Engine.AmbientSound|GetAudioComponent _ambientsoundref))
  (Audio|Parameter|SetFloatParameter _audiocomponent "M_CloseVolume" (Math|Float|Clamp(Float) (/ (- 1.0 (/ (Math|Vector|VectorLength (- (Transformation|GetActorLocation (Variables|Default|GetPlayerRef)) (Transformation|GetActorLocation))) (Variables|Default|GetWanderRadiusMax))) (Variables|Default|GetCloseMusicStartRatio))) :!class /Script/Engine.AudioComponent)
  (bind _output_get (LocalVariables|SetChaseVolume (Math|Float|Clamp(Float) (+ (LocalVariables|GetChaseVolume) (* (LocalVariables|GetChaseFadeSpeed) (Utilities|Time|GetWorldDeltaSeconds) (Utilities|Enum|Equal(Enum) (Variables|Default|GetCurrentState) "NewEnumerator2"))))))
  (Development|PrintString (Utilities|String|ToString(Float) _output_get))
  (Audio|Parameter|SetFloatParameter _audiocomponent "M_ChaseVolume" _output_get :!class /Script/AudioExtensions.AudioParameterControllerInterface))

(fn GenerateWanderLocation
  (bind _returnvalue (Math|Random|RandomFloatinRange 0.0 3.6e+02))
  (bind _wanderradiusmax (Variables|Default|GetWanderRadiusMax))
  (bind _wanderradiusmin (Variables|Default|GetWanderRadiusMin))
  (bind _playerref (Variables|Default|GetPlayerRef))
  (bind _returnvalue_2 (Transformation|GetActorLocation _playerref))
  (bind _returnvalue_3 (Math|Random|RandomFloatinRange _wanderradiusmin _wanderradiusmax))
  (return (+ (* _returnvalue_3 (Math|Trig|Cos(Degrees) _returnvalue)) (.x _returnvalue_2)) (+ (* _returnvalue_3 (Math|Trig|Sin(Degrees) _returnvalue)) (.y _returnvalue_2))))